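; A player controller that opens and closes the dialogue UI for a dialogue system.
; ShowDialogueUI creates a WBP_Dialogue widget bound to the supplied dialogue component, switches to UI-only input with a visible cursor, then calls BeginDialogue on that component.
; HideDialogueUI removes the stored widget if valid and restores game-only input with the cursor hidden.
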(event `self.ShowDialogueUI`
  (params (ComponentToUse :type "DialogueComponent Object Reference"))
  (`KismetSystemLibrary.PrintString` "Debug:Sex")
  (bind _returnvalue (`|CreateWidget` "/Game/Dev_KJH/DialogSystem/WBP_Dialogue.WBP_Dialogue_C" null ComponentToUse))
  (bind _output_get (set `self.CurrentDialogueWidget` _returnvalue))
  (`UserWidget.AddToViewport` _output_get 0)
  (`WidgetBlueprintLibrary.SetInputMode_UIOnlyEx` (`GameplayStatics.GetPlayerController` 0) null)
  (set `self.bShowMouseCursor` true)
  (`DialogueComponent.BeginDialogue` (`/Game/Dev_KJH/DialogSystem/WBP_Dialogue.DialogueComponentRef` _output_get)))

(event `HideDialogueUI`
  (bind _currentdialoguewidget (`self.CurrentDialogueWidget`))
  (`/Engine/EditorBlueprintResources/StandardMacros.IsValid` _currentdialoguewidget
    (:`Is Valid`
      (`Widget.RemoveFromParent` _currentdialoguewidget)
      (`WidgetBlueprintLibrary.SetInputMode_GameOnly` (`GameplayStatics.GetPlayerController` 0))
      (set `self.bShowMouseCursor` false))))

(fn `UserConstructionScript`)