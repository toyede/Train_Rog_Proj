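; Player character for a train shooter, handling weapons, enemy targeting and pause menus.
; BeginPlay spawns inventory weapons on a mesh socket; Swap toggles visibility, while Fire and Reload drive the current weapon with montages, recoil and weapon-based timing.
; A camera trace briefly stores Enemy-tagged hit components, and a helper widens bullet spread when not zooming.
; Debug keys damage player or train, open a UI, and remap Enhanced Input keys.
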(event Input|EnhancedActionEvents|EnhancedInputActionIA_Run
  (params (ActionValue :type Boolean) (ElapsedSeconds :type Float%20%28double-precision%29) (TriggeredSeconds :type Float%20%28double-precision%29) (InputAction :type Input%20Action%20Object%20Reference :default "/Game/LJH/Player_LJH/PlayerInput_LJH/IA_Run.IA_Run")))

(event Input|EnhancedActionEvents|EnhancedInputActionIA_Fire
  (params (ActionValue :type Boolean) (ElapsedSeconds :type Float%20%28double-precision%29) (TriggeredSeconds :type Float%20%28double-precision%29) (InputAction :type Input%20Action%20Object%20Reference :default "/Game/LJH/Player_LJH/PlayerInput_LJH/IA_Fire.IA_Fire"))
  (bind _returnvalue (Game|GetPlayerCharacter 0))
  (if (not (Variables|Default|GetbIsRunning))
    (if (not (Variables|Default|GetReloading))
      (Utilities|FlowControl|DoOnce false :!label _label
        (:Completed
          (if (Variables|Default|GetbIsCrouching)
            (Animation|Montage|MontagePlay (Components|SkeletalMesh|GetAnimInstance (Variables|Character|GetMesh)) "/Game/ArtAsset/Character/Anim_CrouchAndAimAttack_Montage.Anim_CrouchAndAimAttack_Montage" 1.0 "MontageLength" 0.0 true)
            (else
              (Animation|Montage|MontagePlay (Components|SkeletalMesh|GetAnimInstance (Variables|Character|GetMesh)) "/Game/ArtAsset/Character/Anim_Attack_Montage.Anim_Attack_Montage" 1.0 "MontageLength" 0.0 true)))
          (if (Utilities|IsValid (Variables|Default|GetCurrentWeapon))
            (Default|Fire (Variables|Default|GetCurrentWeapon))
            (Pawn|Input|AddControllerPitchInput _returnvalue (Math|Random|RandomFloatinRange -0.1 -0.3))
            (Pawn|Input|AddControllerYawInput _returnvalue (Math|Random|RandomFloatinRange -0.3 0.3))
            (Game|Feedback|ClientStartCameraShake (Game|GetPlayerController 0) "/Game/LJH/Player_LJH/Player_LJH/BP_CameraShake.BP_CameraShake_C" 1.0 "CameraLocal" "0, 0, 0")
            (Utilities|FlowControl|Delay (- (Variables|/Game/LJH/Player_LJH/Player_LJH/Weapons/BP_WeaponBase.BP_WeaponBase_C|GetFirelate (Variables|Default|GetCurrentWeapon)) (Variables|/Script/Train_Rog_Proj.AbilityComponent|GetAttackSpeed (Variables|Default|GetAbilityComponent))))
            (goto _label Reset)))))))

(event Input|EnhancedActionEvents|EnhancedInputActionIA_Reload
  (params (ActionValue :type Boolean) (ElapsedSeconds :type Float%20%28double-precision%29) (TriggeredSeconds :type Float%20%28double-precision%29) (InputAction :type Input%20Action%20Object%20Reference :default "/Game/LJH/Player_LJH/PlayerInput_LJH/IA_Reload.IA_Reload"))
  ;[0.15 0.15 0.15 0.5] 장전
  (Variables|Default|SetReloading true)
  (bind _reloaddelay (Default|ReloadDelay (Variables|Default|GetCurrentWeapon)))
  (Development|PrintString (Utilities|String|ToString(Float) _reloaddelay))
  (bind _returnvalue (Animation|Montage|MontagePlay (Components|SkeletalMesh|GetAnimInstance (Variables|Character|GetMesh)) "/Game/ArtAsset/Character/Anim_StandReload_Montage.Anim_StandReload_Montage" (/ (Variables|/Script/Engine.AnimSequenceBase|GetSequenceLength (Variables|Default|GetReloadTime)) _reloaddelay) "Duration" 0.0 true))
  (Development|PrintString (Utilities|String|ToString(Float) _returnvalue))
  (Development|PrintString "Reload")
  (Utilities|FlowControl|Delay _returnvalue)
  (Default|BulletReload (Variables|Default|GetCurrentWeapon)))

(event Input|EnhancedActionEvents|EnhancedInputActionIA_SetTarget
  (params (ActionValue :type Boolean) (ElapsedSeconds :type Float%20%28double-precision%29) (TriggeredSeconds :type Float%20%28double-precision%29) (InputAction :type Input%20Action%20Object%20Reference :default "/Game/LJH/Player_LJH/PlayerInput_LJH/IA_SetTarget.IA_SetTarget"))
  (bind _followcamera (Variables|Default|GetFollowCamera))
  (bind _returnvalue (Transformation|GetWorldLocation _followcamera))
  ;[0.15 0.15 0.15 0.5] 타겟지정
  (:Started
    (bind (_outhit _returnvalue_2) (Collision|LineTraceByChannel _returnvalue (+ _returnvalue (* (Math|Vector|GetForwardVector _followcamera) 1e+04)) "TraceTypeQuery1" false 0 "ForDuration"))
    (if _returnvalue_2
      (if (Actor|ActorHasTag (.HitActor (Collision|BreakHitResult _outhit)) "Enemy")
        (Variables|Default|SetHit%20Component (.HitComponent (Collision|BreakHitResult _outhit)))
        (Development|PrintString (Utilities|GetDisplayName (Variables|Default|GetHit%20Component)))
        (Utilities|FlowControl|Delay 3.0)
        (Development|PrintString "DelayEnd")
        (Variables|Default|SetHit%20Component (Variables|Default|GetNoneHitComponent))))))

(event Input|EnhancedActionEvents|EnhancedInputActionIA_Pause
  (params (ActionValue :type Boolean) (ElapsedSeconds :type Float%20%28double-precision%29) (TriggeredSeconds :type Float%20%28double-precision%29) (InputAction :type Input%20Action%20Object%20Reference :default "/Game/LJH/Player_LJH/PlayerInput_LJH/IA_Pause.IA_Pause"))
  (bind _returnvalue (Game|GetPlayerController 0))
  (bind _returnvalue_2 (Game|GetPlayerController 0))
  (if (not (Variables|Default|GetIsPaused))
    (Variables|Default|SetIsPaused true)
    (Game|SetGamePaused true)
    (bind _returnvalue_3 (UserInterface|CreateWidget "/Game/LJH/Player_LJH/PlayerUI_LJH/WBP_Stop.WBP_Stop_C"))
    (bind _output_get (Variables|Default|SetPauseMenu _returnvalue_3))
    (Widget|SetKeyboardFocus _returnvalue_3)
    (UserInterface|Viewport|AddtoViewport _returnvalue_3 0)
    (Input|SetInputModeGameandUI _returnvalue _returnvalue_3 "DoNotLock" true false)
    (Variables|/Script/Engine.PlayerController|SetbShowMouseCursor _returnvalue true)
    (else
      (Variables|Default|SetIsPaused false)
      (Game|SetGamePaused false)
      (Variables|/Script/Engine.PlayerController|SetbShowMouseCursor _returnvalue_2 false)
      (Input|SetInputModeGameOnly _returnvalue_2 false)
      (Widget|RemovefromParent (Variables|Default|GetPauseMenu)))))

(event Input|EnhancedActionEvents|EnhancedInputActionIA_Swap
  (params (ActionValue :type Boolean) (ElapsedSeconds :type Float%20%28double-precision%29) (TriggeredSeconds :type Float%20%28double-precision%29) (InputAction :type Input%20Action%20Object%20Reference :default "/Game/LJH/Player_LJH/PlayerInput_LJH/IA_Swap.IA_Swap"))
  ;[0.15 0.15 0.15 0.5] 무기교체
  (if (== (Variables|Default|GetCurrentWeaponIndex) 0)
    (Variables|Default|SetCurrentWeaponIndex 1)
    (else
      (Variables|Default|SetCurrentWeaponIndex 0)))
  (for (_array_element _array_index) (Variables|Default|GetSpawnedWeapons)
    (if (== _array_index (Variables|Default|GetCurrentWeaponIndex))
      (Rendering|SetActorHiddenInGame _array_element false)
      (Variables|Default|SetCurrentWeapon (Utilities|Array|Get(acopy) (Variables|Default|GetSpawnedWeapons) (Variables|Default|GetCurrentWeaponIndex)))
      (else
        (Rendering|SetActorHiddenInGame _array_element true)))))

(event EventBeginPlay
  (bind _spawnedweapons (Variables|Default|GetSpawnedWeapons))
  (bind _output (Utilities|Array|Get(acopy) _spawnedweapons))
  ;[0.15 0.15 0.15 0.5] 플레이어 스폰시
  (bind _returnvalue (UserInterface|CreateWidget (Variables|Default|GetClass)))
  (UserInterface|Viewport|AddtoViewport _returnvalue 0)
  (for (_array_element _array_index) (Variables|Default|GetWeaponInventory)
    (bind _returnvalue_2 (Game|SpawnActorfromClass _array_element (Math|Transform|MakeTransform "0, 0, 0" "0, 0, 0" "1.000000,1.000000,1.000000") "Undefined" "MultiplyWithRoot" 0 0))
    (Utilities|Array|Add (Variables|Default|GetSpawnedWeapons) _returnvalue_2)
    (Transformation|AttachComponentToComponent _returnvalue_2 (Variables|Character|GetMesh) "ShotGun" "SnapToTarget" "SnapToTarget" "KeepRelative" true)
    (Rendering|SetActorHiddenInGame _returnvalue_2 true))
  (Rendering|SetActorHiddenInGame _output false)
  (Variables|Default|SetCurrentWeapon _output))

(event Input|KeyboardEvents|DebugKeyU
  (params (Key :type Key%20Structure :default "None") (ActionValue :type Input%20Action%20Value%20Structure))
  (:Pressed
    (Variables|Default|SetU Key)
    (Variables|Default|SetRemapping true)
    (Variables|Default|SetRemapIndex false)
    (Development|PrintString "Start ReMapKey")))

(event Input|KeyboardEvents|DebugKeyL
  (params (Key :type Key%20Structure :default "None") (ActionValue :type Input%20Action%20Value%20Structure))
  (bind _healthcomponent (Variables|Default|GetHealthComponent))
  (:Pressed
    (Variables|/Script/Train_Rog_Proj.HealthComponent|SetCurrentHP _healthcomponent (- (Variables|/Script/Train_Rog_Proj.HealthComponent|GetCurrentHP _healthcomponent) 1e+01))))

(event Input|KeyboardEvents|DebugKeyP
  (params (Key :type Key%20Structure :default "None") (ActionValue :type Input%20Action%20Value%20Structure))
  (bind _returnvalue (Game|GetPlayerController 0))
  (:Pressed
    (Game|SetGamePaused true)
    (Input|SetInputModeUIOnly _returnvalue 0 "DoNotLock" false)
    (Variables|/Script/Engine.PlayerController|SetbShowMouseCursor _returnvalue true)
    (bind _returnvalue_2 (UserInterface|CreateWidget "/Game/LJH/Player_LJH/PlayerUI_LJH/WBP_Base.WBP_Base_C"))
    (UserInterface|Viewport|AddtoViewport _returnvalue_2 0)))

(event Input|KeyboardEvents|DebugKeyT
  (params (Key :type Key%20Structure :default "None") (ActionValue :type Input%20Action%20Value%20Structure))
  (:Pressed
    (bind _outactors (Actor|GetAllActorsOfClass "/Game/LJH/Train_LJH/BP_Train.BP_Train_C"))
    (Variables|/Script/Train_Rog_Proj.Train|SetCurrentTrainHealth (Utilities|Array|Get(acopy) _outactors) (- (Variables|/Script/Train_Rog_Proj.Train|GetCurrentTrainHealth (Utilities|Array|Get(acopy) _outactors)) 2e+01))))

(event Input|KeyboardEvents|AnyKey
  (params (Key :type Key%20Structure :default "None"))
  (:Pressed
    (if (not (Class|TrainBlueprintFunctionLibrary|IsSameKey Key (Variables|Default|GetU)))
      (if (Variables|Default|GetRemapping)
        (if (Variables|Default|GetRemapIndex)
          (bind _output_get (Variables|Default|SetOldKey Key))
          (bind _returnvalue (Class|TrainBlueprintFunctionLibrary|FindInputActionbyKey "/Game/LJH/Player_LJH/PlayerInput_LJH/IMC_Player.IMC_Player" _output_get))
          (Variables|Default|SetRemapIndex false)
          (Development|PrintString "Select OldKey")
          (else
            (bind _output_get_2 (Variables|Default|SetNewKey Key))
            (Class|TrainCharacter|RemapKey _returnvalue _output_get _output_get_2)
            (Variables|Default|SetRemapping false)
            (Development|PrintString "Change NewKey")))))))

(fn ConstructionScript)

(fn 집탄율
  (params (IsZooming :type Boolean))
  (bind _currentweapon (Variables|Default|GetCurrentWeapon))
  (bind _bulletradious (Variables|/Game/LJH/Player_LJH/Player_LJH/Weapons/BP_WeaponBase.BP_WeaponBase_C|GetBulletRadious _currentweapon))
  (if IsZooming
    (Variables|Default|SetAccumulation%20rate _bulletradious)
    (else
      (bind _output_get (Variables|Default|SetAccumulation%20rate (* _bulletradious 1.5)))))
  (return _output_get))