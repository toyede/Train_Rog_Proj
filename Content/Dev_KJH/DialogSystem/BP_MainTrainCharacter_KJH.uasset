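; Character Blueprint that prototypes magazine-based gun firing on debug keys, with debug prints.
; Left mouse spawns BP_Bullet at the Gun's location along the actor's rotation, adding positive-only random pitch and yaw from 집탄율 (spread, tighter when zooming) divided by MaxDistance.
; R or firing on empty calls Reload, which refills the magazine to 30 after a delay.
; The Reloading flag is inverted: true means ready to fire.
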(event Custom|Reload
  ;[0.15 0.15 0.15 0.5] 장전 함수
  (Variables|Default|SetReloading false)
  (Development|PrintString "Reload")
  (Utilities|FlowControl|Delay 3.0)
  (Development|PrintString "Clear")
  (Variables|Default|SetReloading true)
  (Variables|Default|Setmagazine 30))

(event EventBeginPlay)

(event Collision|EventActorBeginOverlap
  (params (OtherActor :type Actor%20Object%20Reference)))

(event EventTick
  (params (DeltaSeconds :type Float%20%28single-precision%29)))

(event Input|MouseEvents|DebugKeyLeftMouseButton
  (params (Key :type Key%20Structure :default "None") (ActionValue :type Input%20Action%20Value%20Structure))
  (bind _returnvalue (Transformation|GetActorTransform))
  (:Pressed
    (if (> (Variables|Default|Getmagazine) 0)
      (if (Variables|Default|GetReloading)
        (Development|PrintString (Utilities|String|ToString(Integer) (Variables|Default|Getmagazine)))
        (bind _rate (CallFunction|집탄율 (Variables|Default|GetbIsZooming)))
        (Variables|Default|Setmagazine (- (Variables|Default|Getmagazine) 1))
        (Game|SpawnActorfromClass "/Game/LJH/Player_LJH/Player_LJH/BP_Bullet.BP_Bullet_C" (Math|Transform|MakeTransform (Transformation|GetWorldLocation (Variables|컴포넌트|GetGun)) (Math|Rotator|MakeRotator (.roll (.rotation _returnvalue)) (+ (.pitch (.rotation _returnvalue)) (Math|Random|RandomFloatinRange 0.0 (/ _rate (Variables|Default|GetMaxDistance)))) (+ (.yaw (.rotation _returnvalue)) (Math|Random|RandomFloatinRange 0.0 (/ _rate (Variables|Default|GetMaxDistance))))) (.scale _returnvalue)) "Undefined" "MultiplyWithRoot" 0 0)
        (Development|PrintString (Utilities|String|ToString(Float) (Variables|Default|GetAccumulation%20rate)) true true "(R=1.000000,G=0.075130,B=0.000000,A=1.000000)")
        (else
          (Development|PrintString "Reload")))
      (else
        (CallFunction|Reload)))))

(event Input|KeyboardEvents|DebugKeyR
  (params (Key :type Key%20Structure :default "None") (ActionValue :type Input%20Action%20Value%20Structure))
  ;[0.15 0.15 0.15 0.5] R키를 눌러 장전
  (:Pressed
    (CallFunction|Reload)))

(fn ConstructionScript)

(fn 집탄율
  (params (IsZooming :type Boolean))
  (if IsZooming
    (Variables|Default|SetAccumulation%20rate 2e+01)
    (else
      (bind _output_get (Variables|Default|SetAccumulation%20rate 5e+01))))
  (return _output_get))