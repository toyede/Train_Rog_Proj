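; BP_TestTrain is a test train actor that takes damage and is destroyed when its health runs out.
; On BeginPlay it hands its Health component to its WBP_TestHP widget.
; AnyDamage scales incoming damage by a diminishing-returns formula on Ability Defense before reducing HP, and OnDeath destroys the actor.
; Debug prints show current HP, damage taken and destruction, while a movement offset node is left unconnected.
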(event `self.ReceiveBeginPlay`
  (bind _aswbp_test_hp (cast `/Game/JSY/WBP_TestHP` (`WidgetComponent.GetWidget` (`self.Widget`))))
  (set `/Game/JSY/WBP_TestHP.HealthComponent` (`self.Health`) _aswbp_test_hp))

(event `self.ReceiveTick`
  (params (DeltaSeconds :type "Float (single-precision)"))
  (`KismetSystemLibrary.PrintString` (`KismetStringLibrary.Conv_DoubleToString` (`HealthComponent.CurrentHP` (`self.Health`))) true true (struct :`G` 0.66 :`B` 1.0 :`A` 1.0) DeltaSeconds))

(event `self.Health.OnDeath`
  (`KismetSystemLibrary.PrintString` "TRAIN DESTROYED" true true (struct :`R` 1.0 :`B` 0.078098 :`A` 1.0))
  (`self.K2_DestroyActor`))

(event `self.ReceiveAnyDamage`
  (params (Damage :type "Float (single-precision)") (DamageType :type "DamageType Object Reference") (InstigatedBy :type "Controller Object Reference") (DamageCauser :type "Actor Object Reference"))
  (bind _defense (`AbilityComponent.Defense` (`self.Ability`)))
  (bind _returnvalue (* Damage (- 1.0 (/ _defense (+ _defense 2.0)))))
  (`KismetSystemLibrary.PrintString` (`KismetStringLibrary.Concat_StrStr` "DAMEGED BY : " (`KismetSystemLibrary.GetDisplayName` DamageCauser) " || " (`KismetStringLibrary.Conv_DoubleToString` _returnvalue)) true true (struct :`R` 1.0 :`B` 0.011301 :`A` 1.0))
  (`HealthComponent.DecreaseHP` (`self.Health`) _returnvalue))

(fn `UserConstructionScript`)