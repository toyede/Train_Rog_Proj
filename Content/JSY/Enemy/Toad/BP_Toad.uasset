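; BP_Toad is an enemy toad character that attacks a target class and can latch onto trains.
; On BeginPlay it binds its HP bar to HealthComponent and calls FindTarget; death removes the bar and destroys the actor after a delay.
; Attack plays a montage whose notify sphere-traces at the right hand, applying AbilityComponent damage to matching targets.
; TryAttachToTrains jumps, offsets the mesh and attaches the toad to the Blackboard's TargetActor.
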(event `self.ReceiveBeginPlay`
  (bind _aswbp_test_hp (cast `/Game/JSY/WBP_TestHP` (`WidgetComponent.GetWidget` (`self.HPBar`))))
  (set `/Game/JSY/WBP_TestHP.HealthComponent` (`self.HealthComponent`) _aswbp_test_hp)
  (`self.FindTarget`))

(event `self.ReceiveTick`
  (params (DeltaSeconds :type "Float (single-precision)")))

(event `self.HealthComponent.OnDeath`
  (`ActorComponent.K2_DestroyComponent` (`self.HPBar`))
  (`KismetSystemLibrary.Delay` 3.0)
  (`self.K2_DestroyActor`))

(event `self.Attack`
  (bind _returnvalue (`SceneComponent.GetSocketLocation` (`self.Mesh`) "hand_r"))
  (`|PlayMontage` (`self.Mesh`) "/Game/ArtAsset/Monster/Frog/AM_ToadAttack.AM_ToadAttack"
    (:`OnNotifyBegin`
      (bind _outhit (`KismetSystemLibrary.SphereTraceSingle` _returnvalue _returnvalue 20.0 "TraceTypeQuery1" false (`|MakeArray` self :!type "Actor Object Reference")))
      (bind (_bblockinghit _binitialoverlap _time _distance _location _impactpoint _normal _impactnormal _physmat _hitactor) (`GameplayStatics.BreakHitResult` _outhit))
      (if (== (`GameplayStatics.GetObjectClass` _hitactor) (`self.TargetClass`))
        (`GameplayStatics.ApplyDamage` _hitactor (`AbilityComponent.Damage` (`self.AbilityComponent`)) (`self.GetController`) self)))))

(fn `TryAttachToTrains`
  (returns (IsSuccess :type Boolean))
  (`self.Jump`)
  (`SceneComponent.K2_SetRelativeLocation` (`self.Mesh`) (30.0 0.0 -140.0) false false)
  (bind `_as액터` (cast `Actor` (`BlackboardComponent.GetValueAsObject` (`AIBlueprintHelperLibrary.GetBlackboard` (`self.GetController`)) "TargetActor")))
  (bind _returnvalue (`self.K2_AttachToActor` `_as액터` "None" "KeepWorld" "KeepWorld" "KeepWorld" false))
  (return _returnvalue))

(fn `UserConstructionScript`)