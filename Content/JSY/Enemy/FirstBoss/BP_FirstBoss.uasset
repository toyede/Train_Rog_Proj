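; First boss enemy character with an HP bar widget and a child-actor mana core that receives its owner and damage at BeginPlay.
; Fire shot, fan-spread fireball volley and random monster summon functions each gate on a cooldown flag and timer, returning whether they fired.
; Projectiles aim at the player, while summons spawn at random reachable points around the boss.
; Tick prints the Blackboard phase and current HP for debugging; Stun is empty.
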(event `self.ReceiveBeginPlay`
  (bind _aswbp_test_hp (cast `/Game/JSY/WBP_TestHP` (`WidgetComponent.GetWidget` (`self.HPBar`))))
  (set `/Game/JSY/WBP_TestHP.HealthComponent` (`self.HealthComponent`) _aswbp_test_hp)
  (`self.FindTarget`)
  (bind _asbp_mana_core (cast `/Game/JSY/Enemy/FirstBoss/BP_ManaCore` (`ChildActorComponent.ChildActor` (`self.BP_ManaCore`))))
  (set `/Game/JSY/Enemy/FirstBoss/BP_ManaCore.OwnerActor` self _asbp_mana_core)
  (set `/Game/JSY/Enemy/FirstBoss/BP_ManaCore.CoreDamage` (`self.CoreDamage`) _asbp_mana_core))

(event `self.ReceiveTick`
  (params (DeltaSeconds :type "Float (single-precision)"))
  (`KismetSystemLibrary.PrintString` (`|GetEnumeratorNameAsString` (cast `/Game/JSY/Enemy/FirstBoss/E_Phase` (`BlackboardComponent.GetValueAsEnum` (`AIBlueprintHelperLibrary.GetBlackboard` null) "Phase"))) true true (struct :`R` 0.121265 :`G` 1.0 :`A` 1.0) DeltaSeconds)
  (`KismetSystemLibrary.PrintString` (`KismetStringLibrary.Conv_DoubleToString` (`HealthComponent.CurrentHP` (`self.HealthComponent`))) true true (struct :`R` 1.0 :`G` 0.064041 :`A` 1.0) DeltaSeconds))

(event `SetFire`
  (set `self.CanFire` true))

(event `SetSummon`
  (set `self.CanSummon` true))

(event `SetSmash`
  (set `self.CanSmash` true))

(event `SetCrazy`
  (set `self.CanCrazy` true))

(event `Stun`)

(fn `Crazy`
  (params (CoolTime :type "Float (double-precision)"))
  (returns (Result :type Boolean))
  (bind _returnvalue (`SceneComponent.K2_GetComponentLocation` (`self.FirePoint`)))
  (bind (_returnvalue_roll _returnvalue_pitch _returnvalue_yaw) (`KismetMathLibrary.BreakRotator` (`KismetMathLibrary.FindLookAtRotation` _returnvalue (`self.K2_GetActorLocation` (`GameplayStatics.GetPlayerPawn` 0)))))
  (if (`self.CanCrazy`)
    (`KismetSystemLibrary.K2_SetTimerDelegate` (`|CreateDelegate` :!event `SetCrazy`) CoolTime)
    (set `self.CanCrazy` false)
    (for _index (range 21)
      (`|SpawnActorFromClass` "/Game/JSY/Enemy/FirstBoss/BP_BossFire.BP_BossFire_C" (`KismetMathLibrary.MakeTransform` _returnvalue (`KismetMathLibrary.MakeRotator` _returnvalue_roll _returnvalue_pitch (+ (+ -30.0 (* _index (/ 60 20))) _returnvalue_yaw))) "AlwaysSpawn" "MultiplyWithRoot" null 10.0 null))
    (return true)
    (else
      (return false))))

(fn `FireShot`
  (params (CoolTime :type "Float (double-precision)"))
  (returns (Result :type Boolean))
  (bind _returnvalue (`SceneComponent.K2_GetComponentLocation` (`self.FirePoint`)))
  (if (`self.CanFire`)
    (`KismetSystemLibrary.K2_SetTimerDelegate` (`|CreateDelegate` :!event `SetFire`) CoolTime)
    (set `self.CanFire` false)
    (bind _returnvalue_2 (`|SpawnActorFromClass` "/Game/JSY/Enemy/FirstBoss/BP_BossFire.BP_BossFire_C" (`KismetMathLibrary.MakeTransform` _returnvalue (`KismetMathLibrary.FindLookAtRotation` _returnvalue (`self.K2_GetActorLocation` (`GameplayStatics.GetPlayerPawn` 0)))) "AlwaysSpawn" "MultiplyWithRoot" null (`AbilityComponent.Damage` (`self.AbilityComponent`)) null))
    (`PrimitiveComponent.IgnoreActorWhenMoving` (`/Game/JSY/Enemy/FirstBoss/BP_BossFire.Sphere` _returnvalue_2) self true)
    (return true)
    (else
      (return false))))

(fn `SummonMonsters`
  (params (CoolTimes :type "Float (double-precision)"))
  (returns (Result :type Boolean))
  (if (`self.CanSummon`)
    (`KismetSystemLibrary.K2_SetTimerDelegate` (`|CreateDelegate` :!event `SetSummon`) CoolTimes)
    (set `self.CanSummon` false)
    (`self.PlayAnimMontage` "/Game/ArtAsset/Monster/1StageBoss/AM_Anim_1Boss_Summon_Montage.AM_Anim_1Boss_Summon_Montage")
    (for _ (range (+ (+ (`KismetMathLibrary.RandomInteger` 5) 5) 1))
      (`|SpawnActorFromClass` (`self.SummonMonsterClass`) (`KismetMathLibrary.MakeTransform` (`NavigationSystemV1.K2_GetRandomReachablePointInRadius` (`self.K2_GetActorLocation`) 1000.0 null null) (`self.K2_GetActorRotation`)) "AdjustIfPossibleButAlwaysSpawn" "MultiplyWithRoot" null null))
    (return true)
    (else
      (return false))))

(fn `UserConstructionScript`)