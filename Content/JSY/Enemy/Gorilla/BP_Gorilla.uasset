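; BP_Gorilla is a gorilla enemy Blueprint with a health bar and death cleanup.
; On BeginPlay it passes its HealthComponent to the WBP_TestHP widget in HPBar, then calls FindTarget, which is not defined in this graph.
; When HealthComponent fires OnDeath, it destroys the HP bar and removes the actor after a short delay.
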(event `self.ReceiveBeginPlay`
  (bind _aswbp_test_hp (cast `/Game/JSY/WBP_TestHP` (`WidgetComponent.GetWidget` (`self.HPBar`))))
  (set `/Game/JSY/WBP_TestHP.HealthComponent` (`self.HealthComponent`) _aswbp_test_hp)
  (`self.FindTarget`))

(event `self.ReceiveTick`
  (params (DeltaSeconds :type "Float (single-precision)")))

(event `self.HealthComponent.OnDeath`
  (`ActorComponent.K2_DestroyComponent` (`self.HPBar`))
  (`KismetSystemLibrary.Delay` 3.0)
  (`self.K2_DestroyActor`))

(fn `UserConstructionScript`)