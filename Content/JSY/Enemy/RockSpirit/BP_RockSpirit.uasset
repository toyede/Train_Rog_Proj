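; Rock Spirit enemy character that can leap onto a target, apparently a train, and attach itself to it.
; On BeginPlay it links its HP bar widget to the HealthComponent and calls FindTarget.
; TryAttachToTrains jumps, plays a frog jump animation, offsets the mesh and snaps the actor onto the AI blackboard's TargetActor.
; On death it removes the HP bar and destroys itself after a short delay.
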(event `self.ReceiveBeginPlay`
  (bind _aswbp_test_hp (cast `/Game/JSY/WBP_TestHP` (`WidgetComponent.GetWidget` (`self.HPBar`))))
  (set `/Game/JSY/WBP_TestHP.HealthComponent` (`self.HealthComponent`) _aswbp_test_hp)
  (`self.FindTarget`))

(event `self.ReceiveTick`
  (params (DeltaSeconds :type "Float (single-precision)")))

(event `self.HealthComponent.OnDeath`
  (`ActorComponent.K2_DestroyComponent` (`self.HPBar`))
  (`KismetSystemLibrary.Delay` 3.0)
  (`self.K2_DestroyActor`))

(fn `TryAttachToTrains`
  (returns (IsSuccess :type Boolean))
  (`self.Jump`)
  (`SkeletalMeshComponent.PlayAnimation` (`self.Mesh`) "/Game/ArtAsset/Monster/Frog/frog_Anim_jump.frog_Anim_jump" false)
  (`SceneComponent.K2_SetRelativeLocation` (`self.Mesh`) (30.0 0.0 -140.0) false false)
  (bind `_as액터` (cast `Actor` (`BlackboardComponent.GetValueAsObject` (`AIBlueprintHelperLibrary.GetBlackboard` (`self.GetController`)) "TargetActor")))
  (bind _returnvalue (`self.K2_AttachToActor` `_as액터` "None" "SnapToTarget" "KeepRelative" "KeepWorld"))
  (return _returnvalue))

(fn `UserConstructionScript`)