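; BP_Moth is a moth enemy that attacks its target with homing projectiles.
; BeginPlay binds the health component to the HP bar widget and calls FindTarget.
; Attack plays a montage whose notify calls Fire, spawning a BP_MothBullet at FirePoint, aimed at the target and homing on its root component.
; On death it removes the HP bar and waits briefly, but DestroyActor is disconnected, so this graph never destroys the actor.
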(event `self.ReceiveBeginPlay`
  (bind _aswbp_test_hp (cast `/Game/JSY/WBP_TestHP` (`WidgetComponent.GetWidget` (`self.HPBar`))))
  (set `/Game/JSY/WBP_TestHP.HealthComponent` (`self.HealthComponent`) _aswbp_test_hp)
  (`self.FindTarget`))

(event `self.ReceiveTick`
  (params (DeltaSeconds :type "Float (single-precision)")))

(event `self.HealthComponent.OnDeath`
  (`ActorComponent.K2_DestroyComponent` (`self.HPBar`))
  (`KismetSystemLibrary.Delay` 3.0))

(event `self.Attack`
  (`|PlayMontage` (`self.Mesh`) "/Game/ArtAsset/Monster/Moth/AM_MothAttack.AM_MothAttack"
    (:`OnNotifyBegin`
      (`self.Fire`))))

(event `Fire`
  (bind (_returnvalue_location _returnvalue_rotation _returnvalue_scale) (`KismetMathLibrary.BreakTransform` (`SceneComponent.K2_GetComponentToWorld` (`self.FirePoint`))))
  (bind _returnvalue (`|SpawnActorFromClass` "/Game/JSY/Enemy/Moth/BP_MothBullet.BP_MothBullet_C" (`KismetMathLibrary.MakeTransform` _returnvalue_location (`KismetMathLibrary.FindLookAtRotation` (`self.K2_GetActorLocation`) (`self.K2_GetActorLocation` (`self.Target`))) _returnvalue_scale) "AlwaysSpawn" "MultiplyWithRoot" null self null))
  (set `ProjectileMovementComponent.HomingTargetComponent` (`Actor.RootComponent` (`self.Target`)) (`/Game/JSY/Enemy/Moth/BP_MothBullet.ProjectileMovement` _returnvalue)))

(fn `UserConstructionScript`)