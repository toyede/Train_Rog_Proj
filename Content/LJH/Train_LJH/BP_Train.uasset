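; BP_Train is a train actor that builds its attached cars and initializes its stats when play begins.
; It spawns BP_PlusTrain actors in a loop driven by a hardcoded TrainStack, socketing the first to its own mesh and each next one to the previous car's mesh via LastTrain.
; TrainStack then feeds the health and defense increase calls, and current health is set to TrainHealth.
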(event `self.ReceiveBeginPlay`
  (bind _trainstack (`self.TrainStack`))
  (set `self.TrainStack` 1)
  (for _index (range (+ (`self.TrainStack`) 1))
    (if (== _index 0)
      (bind _returnvalue (`|SpawnActorFromClass` "/Game/LJH/Train_LJH/BP_PlusTrain.BP_PlusTrain_C" (`KismetMathLibrary.MakeTransform` (0.0 0.0 0.0)) "Undefined" "MultiplyWithRoot" null null))
      (bind _output_get (set `self.LastTrain` _returnvalue))
      (`self.K2_AttachToComponent` _output_get (`self.StaticMesh`) "PlusTrain" "KeepRelative" "KeepRelative" "KeepRelative" true)
      (else
        (bind _returnvalue_2 (`|SpawnActorFromClass` "/Game/LJH/Train_LJH/BP_PlusTrain.BP_PlusTrain_C" (`KismetMathLibrary.MakeTransform` (0.0 0.0 0.0)) "Undefined" "MultiplyWithRoot" null null))
        (`self.K2_AttachToComponent` _returnvalue_2 (`/Game/LJH/Train_LJH/BP_PlusTrain.StaticMesh` (`self.LastTrain`)) "PlusTrains" "KeepRelative" "KeepRelative" "KeepRelative" true)
        (set `self.LastTrain` _returnvalue_2))))
  (`self.IncreaseTrainHealth` _trainstack)
  (`self.IncreaseTrainDefense` _trainstack)
  (set `self.CurrentTrainHealth` (`self.TrainHealth`)))

(fn `UserConstructionScript`)