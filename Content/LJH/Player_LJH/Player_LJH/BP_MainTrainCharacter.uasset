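; Player character that carries a set of weapons and handles firing, reloading, swapping and enemy targeting.
; BeginPlay adds the HUD, fills HP and spawns every inventory weapon on the hand socket, showing only the first.
; Swap cycles weapons by toggling visibility, while fire and delayed reload call the current weapon.
; Targeting traces from the camera, briefly storing the hit component of Enemy-tagged actors; a helper returns spread by zoom state.
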(event `self.ReceiveBeginPlay`
  (bind _output (`|GetArrayItem` (`self.SpawnedWeapons`)))
  ; 플레이어 스폰시
  (bind _returnvalue (`|CreateWidget` "/Game/LJH/Player_LJH/Player_LJH/WBP_UI.WBP_UI_C"))
  (`UserWidget.AddToViewport` _returnvalue 0)
  (set `self.HP` (`self.MaxHP`))
  (for _array_element (`self.WeaponInventory`)
    (bind _returnvalue_2 (`|SpawnActorFromClass` _array_element (`KismetMathLibrary.MakeTransform` (0.0 0.0 0.0)) "Undefined" "MultiplyWithRoot" null null))
    (`KismetArrayLibrary.Array_Add` (`self.SpawnedWeapons`) _returnvalue_2)
    (`self.K2_AttachToComponent` _returnvalue_2 (`self.Mesh`) "Weapon_r" "SnapToTarget" "SnapToTarget" "KeepRelative" true)
    (`self.SetActorHiddenInGame` _returnvalue_2 true))
  (`self.SetActorHiddenInGame` _output false)
  (set `self.CurrentWeapon` _output))

(event `EnhancedInput|/Game/LJH/Player_LJH/PlayerInput_LJH/IA_Reload`
  (params (ActionValue :type Boolean) (ElapsedSeconds :type "Float (double-precision)") (TriggeredSeconds :type "Float (double-precision)") (InputAction :type "InputAction Object Reference" :default "/Game/LJH/Player_LJH/PlayerInput_LJH/IA_Reload.IA_Reload"))
  ; R키를 눌러 장전
  (:`Triggered`
    (`KismetSystemLibrary.PrintString` "Reload")
    (`KismetSystemLibrary.Delay` 2.0)
    (`/Game/LJH/Player_LJH/Player_LJH/Weapons/BP_WeaponBase.BulletReload` (`self.CurrentWeapon`))))

(event `EnhancedInput|/Game/LJH/Player_LJH/PlayerInput_LJH/IA_Fire`
  (params (ActionValue :type Boolean) (ElapsedSeconds :type "Float (double-precision)") (TriggeredSeconds :type "Float (double-precision)") (InputAction :type "InputAction Object Reference" :default "/Game/LJH/Player_LJH/PlayerInput_LJH/IA_Fire.IA_Fire"))
  ; 발사
  (:`Triggered`
    (if (`KismetSystemLibrary.IsValid` (`self.CurrentWeapon`))
      (`/Game/LJH/Player_LJH/Player_LJH/Weapons/BP_WeaponBase.Fire` (`self.CurrentWeapon`)))))

(event `EnhancedInput|/Game/LJH/Player_LJH/PlayerInput_LJH/IA_Swap`
  (params (ActionValue :type Boolean) (ElapsedSeconds :type "Float (double-precision)") (TriggeredSeconds :type "Float (double-precision)") (InputAction :type "InputAction Object Reference" :default "/Game/LJH/Player_LJH/PlayerInput_LJH/IA_Swap.IA_Swap"))
  (bind _currentweaponindex (`self.CurrentWeaponIndex`))
  (bind _returnvalue (+ (`self.CurrentWeaponIndex`) 1))
  ; 무기교체
  (:`Triggered`
    (if (> (`KismetArrayLibrary.Array_Length` (`self.SpawnedWeapons`)) _returnvalue)
      (set `self.CurrentWeaponIndex` _returnvalue)
      (else
        (set `self.CurrentWeaponIndex` 0)))
    (for (_array_element _array_index) (`self.SpawnedWeapons`)
      (if (== _array_index _currentweaponindex)
        (`self.SetActorHiddenInGame` _array_element false)
        (set `self.CurrentWeapon` (`|GetArrayItem` (`self.SpawnedWeapons`) _currentweaponindex))
        (else
          (`self.SetActorHiddenInGame` _array_element true))))))

(event `EnhancedInput|/Game/LJH/Player_LJH/PlayerInput_LJH/IA_SetTarget`
  (params (ActionValue :type Boolean) (ElapsedSeconds :type "Float (double-precision)") (TriggeredSeconds :type "Float (double-precision)") (InputAction :type "InputAction Object Reference" :default "/Game/LJH/Player_LJH/PlayerInput_LJH/IA_SetTarget.IA_SetTarget"))
  (bind _followcamera (`self.FollowCamera`))
  (bind _returnvalue (`SceneComponent.K2_GetComponentLocation` _followcamera))
  ; 타겟지정
  (:`Started`
    (bind (_outhit _returnvalue_2) (`KismetSystemLibrary.LineTraceSingle` :`Start` _returnvalue :`End` (+ _returnvalue (* (`SceneComponent.GetForwardVector` _followcamera) 10000.0)) :`TraceChannel` "TraceTypeQuery1" :`DrawDebugType` "ForDuration"))
    (if _returnvalue_2
      (bind (_bblockinghit _binitialoverlap _time _distance _location _impactpoint _normal _impactnormal _physmat _hitactor _hitcomponent) (`GameplayStatics.BreakHitResult` _outhit))
      (if (`self.ActorHasTag` _hitactor "Enemy")
        (set `self.Hit Component` _hitcomponent)
        (`KismetSystemLibrary.PrintString` (`KismetSystemLibrary.GetDisplayName` (`self.Hit Component`)))
        (`KismetSystemLibrary.Delay` 3.0)
        (`KismetSystemLibrary.PrintString` "DelayEnd")
        (set `self.Hit Component` (`self.NoneHitComponent`))))))

(fn `UserConstructionScript`)

(fn `집탄율`
  (params (IsZooming :type Boolean))
  (returns (Rate :type "Float (double-precision)"))
  (if IsZooming
    (set `self.Accumulation rate` 1.0)
    (else
      (bind _output_get (set `self.Accumulation rate` 1.5))))
  (return _output_get))