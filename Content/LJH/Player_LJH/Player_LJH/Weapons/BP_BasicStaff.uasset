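; BP_BasicStaff is a staff weapon whose overridden Fire launches magic projectiles for the player's BP_MainTrainCharacter.
; Each shot spawns at a randomized offset ahead of, above and beside the character, rotated toward a point along the camera's forward vector.
; A valid HitComponent on the character makes it spawn BP_BasicMagicBullet homing on that component.
; Otherwise it spawns BulletClass unguided; that branch's camera line trace result is unused.
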(event `self.ReceiveBeginPlay`
  (`parent.ReceiveBeginPlay`))

(fn `Fire`
  (bind _returnvalue (`GameplayStatics.GetPlayerCameraManager` 0))
  (bind _returnvalue_2 (`GameplayStatics.GetPlayerCameraManager` 0))
  (bind _spawnloaction (`self.SpawnLoaction`))
  (bind _returnvalue_3 (`PlayerCameraManager.GetCameraLocation` _returnvalue_2))
  (bind _returnvalue_4 (+ _returnvalue_3 (* (`KismetMathLibrary.GetForwardVector` (`PlayerCameraManager.GetCameraRotation` _returnvalue_2)) (`self.Length`))))
  (bind (_returnvalue_roll _returnvalue_pitch _returnvalue_yaw) (`KismetMathLibrary.BreakRotator` (`KismetMathLibrary.FindLookAtRotation` _spawnloaction _returnvalue_4)))
  (`parent.Fire`)
  (bind _asbp_main_train_character (cast `/Game/LJH/Player_LJH/Player_LJH/BP_MainTrainCharacter` (`GameplayStatics.GetPlayerCharacter` 0)))
  (set `self.LookAtTarget` (+ (`PlayerCameraManager.GetCameraLocation` _returnvalue) (* (`KismetMathLibrary.GetForwardVector` (`PlayerCameraManager.GetCameraRotation` _returnvalue)) (`self.Length`))))
  (bind _returnvalue_5 (`SceneComponent.GetRightVector` (`Character.CapsuleComponent` _asbp_main_train_character)))
  (bind _output_get (set `self.SpawnLoaction` (+ (`self.K2_GetActorLocation` _asbp_main_train_character) (* (`SceneComponent.GetForwardVector` (`Character.CapsuleComponent` _asbp_main_train_character)) (`KismetMathLibrary.RandomFloatInRange` 100.0 500.0)) (* (`SceneComponent.GetUpVector` (`Character.CapsuleComponent` _asbp_main_train_character)) (`KismetMathLibrary.RandomFloatInRange` 100.0 200.0)) (* _returnvalue_5 (`KismetMathLibrary.RandomFloatInRange` 100.0 500.0)) (* _returnvalue_5 (`KismetMathLibrary.RandomFloatInRange` -100.0 -500.0)))))
  (if (`KismetSystemLibrary.IsValid` (`/Game/LJH/Player_LJH/Player_LJH/BP_MainTrainCharacter.Hit Component` _asbp_main_train_character))
    (`KismetSystemLibrary.PrintString` "Horming")
    (bind _returnvalue_6 (`|SpawnActorFromClass` "/Game/LJH/Player_LJH/Player_LJH/Weapons/BP_BasicMagicBullet.BP_BasicMagicBullet_C" (`KismetMathLibrary.MakeTransform` _output_get (`KismetMathLibrary.FindLookAtRotation` _output_get (`self.LookAtTarget`))) "Undefined" "MultiplyWithRoot" null null))
    (bind _asbp_main_train_character_2 (cast `/Game/LJH/Player_LJH/Player_LJH/BP_MainTrainCharacter` (`GameplayStatics.GetPlayerCharacter` 0)))
    (set `ProjectileMovementComponent.HomingTargetComponent` (`/Game/LJH/Player_LJH/Player_LJH/BP_MainTrainCharacter.Hit Component` _asbp_main_train_character_2) (`/Game/LJH/Player_LJH/Player_LJH/Weapons/BP_BasicMagicBullet.ProjectileMovement` _returnvalue_6))
    (else
      (cast `/Game/LJH/Player_LJH/Player_LJH/BP_MainTrainCharacter` (`GameplayStatics.GetPlayerCharacter` 0))
      (`KismetSystemLibrary.LineTraceSingle` _returnvalue_3 _returnvalue_4 "TraceTypeQuery1")
      (`|SpawnActorFromClass` (`self.Bullet Class`) (`KismetMathLibrary.MakeTransform` _spawnloaction (`KismetMathLibrary.MakeRotator` _returnvalue_roll _returnvalue_pitch _returnvalue_yaw)) "Undefined" "MultiplyWithRoot" null null))))

(fn `UserConstructionScript`
  (`parent.UserConstructionScript`))