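; BP_BasicMagicBullet is a player magic projectile that can home in on actors tagged "Enemy".
; On BeginPlay it stores the BP_MainTrainCharacter's HitComponent as TargetEnemy, without assigning it as the homing target.
; If TargetEnemy is invalid, a Sphere2 overlap with an enemy sets that component as the ProjectileMovement homing target.
; A Sphere1 overlap with any enemy prints "Boom" and destroys the bullet, applying no damage.
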(event `self.ReceiveBeginPlay`
  (bind _asbp_main_train_character (cast `/Game/LJH/Player_LJH/Player_LJH/BP_MainTrainCharacter` (`GameplayStatics.GetPlayerCharacter` 0)))
  (set `self.TargetEnemy` (`/Game/LJH/Player_LJH/Player_LJH/BP_MainTrainCharacter.Hit Component` _asbp_main_train_character)))

(event `self.ReceiveTick`
  (params (DeltaSeconds :type "Float (single-precision)")))

(event `self.Sphere2.OnComponentBeginOverlap`
  (params (OverlappedComponent :type "PrimitiveComponent Object Reference") (OtherActor :type "Actor Object Reference") (OtherComp :type "PrimitiveComponent Object Reference") (OtherBodyIndex :type Integer) (bFromSweep :type Boolean) (SweepResult :type "HitResult Structure (by ref)"))
  (if (`KismetSystemLibrary.IsValid` (`self.TargetEnemy`))
    _
    (elif (`self.ActorHasTag` OtherActor "Enemy")
      (bind _output_get (set `self.TargetEnemy` OtherComp))
      (bind _output_get_2 (set `self.HomingTarget` _output_get))
      (set `ProjectileMovementComponent.HomingTargetComponent` _output_get_2 (`self.ProjectileMovement`)))))

(event `self.Sphere1.OnComponentBeginOverlap`
  (params (OverlappedComponent :type "PrimitiveComponent Object Reference") (OtherActor :type "Actor Object Reference") (OtherComp :type "PrimitiveComponent Object Reference") (OtherBodyIndex :type Integer) (bFromSweep :type Boolean) (SweepResult :type "HitResult Structure (by ref)"))
  (if (`self.ActorHasTag` OtherActor "Enemy")
    (`KismetSystemLibrary.PrintString` "Boom")
    (`self.K2_DestroyActor`)))

(fn `UserConstructionScript`)