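; BP_BasicBullet is the player's basic projectile, which damages actors tagged Enemy.
; Each tick it sweeps forward at the current weapon's BulletSpeed, read from BP_MainTrainCharacter, and destroys itself past MaxDistance.
; On sphere overlap with an Enemy, it gets damage from the character's TakeDamage function using weapon damage and crit stats, applies it, then destroys itself.
; The EnemyTakeDamage function is an empty stub.
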(event `self.ReceiveBeginPlay`
  (set `self.BaseLocation` (`self.K2_GetActorLocation`)))

(event `self.ReceiveTick`
  (params (DeltaSeconds :type "Float (single-precision)"))
  (bind _asbp_main_train_character (cast `/Game/LJH/Player_LJH/Player_LJH/BP_MainTrainCharacter` (`GameplayStatics.GetPlayerCharacter` 0)))
  (bind _returnvalue (* DeltaSeconds (`/Game/LJH/Player_LJH/Player_LJH/Weapons/BP_WeaponBase.BulletSpeed` (`/Game/LJH/Player_LJH/Player_LJH/BP_MainTrainCharacter.CurrentWeapon` _asbp_main_train_character))))
  (`self.K2_AddActorLocalOffset` (`KismetMathLibrary.MakeVector` _returnvalue) true)
  (set `self.Distance` (+ (`self.Distance`) _returnvalue))
  (if (> (`self.Distance`) (`self.MaxDistance`))
    (`self.K2_DestroyActor`)))

(event `self.Sphere1.OnComponentBeginOverlap`
  (params (OverlappedComponent :type "PrimitiveComponent Object Reference") (OtherActor :type "Actor Object Reference") (OtherComp :type "PrimitiveComponent Object Reference") (OtherBodyIndex :type Integer) (bFromSweep :type Boolean) (SweepResult :type "HitResult Structure (by ref)"))
  (bind _asbp_main_train_character (cast `/Game/LJH/Player_LJH/Player_LJH/BP_MainTrainCharacter` (`GameplayStatics.GetPlayerCharacter` 0)))
  (if (`self.ActorHasTag` OtherActor "Enemy")
    (bind _asenemy (cast `Enemy` OtherActor))
    (bind _currentweapon (`/Game/LJH/Player_LJH/Player_LJH/BP_MainTrainCharacter.CurrentWeapon` _asbp_main_train_character))
    (bind _returnvalue (`TrainCharacter.TakeDamage` _asbp_main_train_character (`/Game/LJH/Player_LJH/Player_LJH/Weapons/BP_WeaponBase.Damage` _currentweapon) (`/Game/LJH/Player_LJH/Player_LJH/Weapons/BP_WeaponBase.WeaponConst` _currentweapon) (`/Game/LJH/Player_LJH/Player_LJH/Weapons/BP_WeaponBase.CriChance` _currentweapon) (`/Game/LJH/Player_LJH/Player_LJH/Weapons/BP_WeaponBase.CriDam` _currentweapon) true))
    (`GameplayStatics.ApplyDamage` _asenemy _returnvalue (`GameplayStatics.GetPlayerController` 0) _asbp_main_train_character)
    (`self.K2_DestroyActor`)))

(fn `EnemyTakeDamage`
  (params (self2 :type "Actor Object Reference") (InputPin :type "Actor Object Reference")))

(fn `UserConstructionScript`)