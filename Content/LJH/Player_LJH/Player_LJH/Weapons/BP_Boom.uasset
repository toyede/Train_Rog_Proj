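; BP_Boom is an explosive weapon actor that damages enemies entering its BoomArea collision.
; On overlap with an actor tagged Enemy, it subtracts BoomDamage, read from the player character's current weapon, directly from BP_TestEnemy's CurrentHP.
; It prints the new HP and destroys itself, so only BP_TestEnemy actors are affected.
; The Boom component's overlap event, BeginPlay, Tick and construction script are empty.
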(event `self.Boom.OnComponentBeginOverlap`
  (params (OverlappedComponent :type "PrimitiveComponent Object Reference") (OtherActor :type "Actor Object Reference") (OtherComp :type "PrimitiveComponent Object Reference") (OtherBodyIndex :type Integer) (bFromSweep :type Boolean) (SweepResult :type "HitResult Structure (by ref)")))

(event `self.BoomArea.OnComponentBeginOverlap`
  (params (OverlappedComponent :type "PrimitiveComponent Object Reference") (OtherActor :type "Actor Object Reference") (OtherComp :type "PrimitiveComponent Object Reference") (OtherBodyIndex :type Integer) (bFromSweep :type Boolean) (SweepResult :type "HitResult Structure (by ref)"))
  (bind _asbp_main_train_character (cast `/Game/LJH/Player_LJH/Player_LJH/BP_MainTrainCharacter` (`GameplayStatics.GetPlayerCharacter` 0)))
  (if (`self.ActorHasTag` OtherActor "Enemy")
    (bind _asbp_test_enemy (cast `/Game/LJH/Player_LJH/Player_LJH/Weapons/BP_TestEnemy` OtherActor))
    (bind _output_get (set `/Game/LJH/Player_LJH/Player_LJH/Weapons/BP_TestEnemy.CurrentHP` (- (`/Game/LJH/Player_LJH/Player_LJH/Weapons/BP_TestEnemy.CurrentHP` _asbp_test_enemy) (`/Game/LJH/Player_LJH/Player_LJH/Weapons/BP_WeaponBase.BoomDamage` (`/Game/LJH/Player_LJH/Player_LJH/BP_MainTrainCharacter.CurrentWeapon` _asbp_main_train_character))) _asbp_test_enemy))
    (`KismetSystemLibrary.PrintString` (`KismetStringLibrary.Conv_DoubleToString` _output_get))
    (`self.K2_DestroyActor`)))

(fn `UserConstructionScript`)