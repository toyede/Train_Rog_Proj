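; BP_BasicGun is a player gun that fires projectiles from its muzzle toward the camera's aim point, extending a parent weapon's functions.
; Fire checks Magazine and the Reloading flag, decrements ammo and spawns a bullet with random pitch/yaw spread from BP_MainTrainCharacter's zoom-dependent 집탄율.
; The aim point is camera forward times Length; the line trace result is unused.
; An empty magazine triggers OverReload, which waits ReloadDelay before BulletReload refills to MaxMagazine.
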(event `self.ReceiveBeginPlay`
  (`parent.ReceiveBeginPlay`))

(event `overReload`
  (bind _reloaddelay (`self.ReloadDelay`))
  (`KismetSystemLibrary.Delay` _reloaddelay)
  (`self.BulletReload`))

(fn `BulletReload`
  (set `self.magazine` (`self.MaxMagazine`))
  (`KismetSystemLibrary.PrintString` "Reload Clear"))

(fn `Fire`
  (bind _returnvalue (`GameplayStatics.GetPlayerCameraManager` 0))
  (bind _returnvalue_2 (`SceneComponent.GetSocketLocation` (`self.Muzzle`) "None"))
  (bind _returnvalue_3 (`PlayerCameraManager.GetCameraLocation` _returnvalue))
  (bind _returnvalue_4 (+ _returnvalue_3 (* (`KismetMathLibrary.GetForwardVector` (`PlayerCameraManager.GetCameraRotation` _returnvalue)) (`self.Length`))))
  (bind (_returnvalue_roll _returnvalue_pitch _returnvalue_yaw) (`KismetMathLibrary.BreakRotator` (`KismetMathLibrary.FindLookAtRotation` _returnvalue_2 _returnvalue_4)))
  (`parent.Fire`)
  (if (> (`self.magazine`) 0)
    (if (`self.Reloading`)
      (bind _asbp_main_train_character (cast `/Game/LJH/Player_LJH/Player_LJH/BP_MainTrainCharacter` (`GameplayStatics.GetPlayerCharacter` 0)))
      (bind _rate (`/Game/LJH/Player_LJH/Player_LJH/BP_MainTrainCharacter.집탄율` _asbp_main_train_character (`TrainCharacter.bIsZooming` _asbp_main_train_character)))
      (`KismetSystemLibrary.LineTraceSingle` _returnvalue_3 _returnvalue_4 "TraceTypeQuery1")
      (set `self.magazine` (- (`self.magazine`) 1))
      (bind _returnvalue_5 (* _rate -1.0))
      (`|SpawnActorFromClass` (`self.BulletClass`) (`KismetMathLibrary.MakeTransform` _returnvalue_2 (`KismetMathLibrary.MakeRotator` _returnvalue_roll (+ _returnvalue_pitch (`KismetMathLibrary.RandomFloatInRange` _returnvalue_5 _rate)) (+ _returnvalue_yaw (`KismetMathLibrary.RandomFloatInRange` _returnvalue_5 _rate)))) "Undefined" "MultiplyWithRoot" null null))
    (else
      (`self.overReload`))))

(fn `ReloadDelay`
  (returns (ReloadDelay :type "Float (double-precision)"))
  (locals (ReDelay :type "Float (double-precision)" :default 2.0))
  (`parent.ReloadDelay`)
  (bind _output_get (set `self.ReloadingDelay` (`local.ReDelay`)))
  (return _output_get))

(fn `UserConstructionScript`
  (`parent.UserConstructionScript`))