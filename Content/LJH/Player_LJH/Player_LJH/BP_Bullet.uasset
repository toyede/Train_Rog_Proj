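; BP_Bullet is a bullet projectile actor that flies straight along its local X axis until it exceeds a maximum range.
; Each Tick moves it by Speed scaled by delta time with sweep enabled, adds that step to Distance, and destroys it past MaxDistance.
; Range counts requested movement rather than actual displacement, so the BaseLocation stored at BeginPlay goes unused.
; The graph contains no hit or damage handling.
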(event `self.ReceiveBeginPlay`
  (set `self.BaseLocation` (`self.K2_GetActorLocation`)))

(event `self.ReceiveTick`
  (params (DeltaSeconds :type "Float (single-precision)"))
  (bind _returnvalue (* DeltaSeconds (`self.Speed`)))
  (`self.K2_AddActorLocalOffset` (`KismetMathLibrary.MakeVector` _returnvalue) true)
  (set `self.Distance` (+ (`self.Distance`) _returnvalue))
  (if (> (`self.Distance`) (`self.MaxDistance`))
    (`self.K2_DestroyActor`)))

(fn `UserConstructionScript`)